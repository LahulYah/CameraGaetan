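; A camera trigger actor that takes over the third-person character's follow camera when the character enters its box.
; On overlap it clears the character's HaveCameraControl flag and plays a timeline that blends the camera toward the Target actor's transform.
; A second timeline track rotates the camera to look at the trigger actor.
; Both blends lerp from the camera's current values each update, and no end-overlap logic restores control.
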(event OnComponentBeginOverlap(Box)
  (params (OverlappedComponent :type Primitive%20Component%20Object%20Reference) (OtherActor :type Actor%20Object%20Reference) (OtherComp :type Primitive%20Component%20Object%20Reference) (OtherBodyIndex :type Integer) (bFromSweep :type Boolean) (SweepResult :type Hit%20Result%20Structure%20%28by%20ref%29))
  (bind _character (Variables|Default|GetCharacter))
  (bind _followcamera (Variables|/Game/ThirdPerson/Blueprints/BP_ThirdPersonCharacter.BP_ThirdPersonCharacter_C|GetFollowCamera _character))
  (Utilities|Casting|CastToBP_ThirdPersonCharacter OtherActor)
  (Variables|/Game/ThirdPerson/Blueprints/BP_ThirdPersonCharacter.BP_ThirdPersonCharacter_C|SethaveCameraControl (Variables|Default|GetCharacter) false)
  (bind (_direction _output _rotation) (Timeline|Timeline_0 Play)
    (:Update
      (Transformation|SetWorldTransform _followcamera (Math|Transform|Lerp(Transform) (Transformation|GetWorldTransform _followcamera) (Transformation|GetWorldTransform (Variables|/Script/Engine.Actor|GetRootComponent (Variables|Default|GetTarget))) _output) false false)
      (Transformation|SetWorldRotation _followcamera (Math|Rotator|Lerp(Rotator) (Transformation|GetWorldRotation _followcamera) (Math|Rotator|FindLookatRotation (Transformation|GetWorldLocation _followcamera) (Transformation|GetActorLocation)) _rotation) false false))))

(fn ConstructionScript)